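; Interactable wave-start actor, apparently a pillar, that tells HeroGameMode to begin enemy or gameplay waves.
; Interact calls StartWave at WaveLevel 1 or below, otherwise StartsNewWave, and also spawns a weapon if the level then equals four.
; MovePilarDown alternates between two timelines that drive the root's height at a hardcoded XY position.
; MovePilarUp is empty, and nothing in this graph calls the movement events.
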(event Custom|MovePilarDown
  (Utilities|FlowControl|FlipFlop
    (:A
      (bind _newtrack_0 (Timeline|Timeline_0 PlayFromStart)
        (:Update
          (Transformation|SetRelativeLocation (Variables|Default|GetDefaultSceneRoot) (Math|Vector|MakeVector -3.1e+02 2.03e+03 _newtrack_0) false false))))
    (:B
      (bind _newtrack_0_2 (Timeline|Timeline_1 PlayFromStart)
        (:Update
          (Transformation|SetRelativeLocation (Variables|Default|GetDefaultSceneRoot) (Math|Vector|MakeVector -3.1e+02 2.03e+03 _newtrack_0_2) false false))))))

(event Custom|MovePilarUp)

(event EventInteract
  (bind _ashero_game_mode (Utilities|Casting|CastToHeroGameMode (Game|GetGameMode)))
  (bind _output_get (Variables|Default|SetGameModeRef _ashero_game_mode))
  (if (> (Variables|/Script/Soldier.Hero_GameMode|GetWaveLevel _output_get) 1)
    (Default|StartsNewWave _output_get)
    (if (== (Variables|/Script/Soldier.Hero_GameMode|GetWaveLevel _output_get) 4)
      (Default|SpawnWeapon _output_get))
    (else
      (Default|StartWave _output_get))))

(fn ConstructionScript)