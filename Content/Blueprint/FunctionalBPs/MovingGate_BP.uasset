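; MovingGate_BP is a gate that alternates between two vertical movements each time its MoveGate event fires.
; A FlipFlop plays one of two timelines from the start, and each timeline drives the static mesh's relative Z.
; The relative X and Y are hardcoded constants.
; BeginPlay caches the HeroGameMode, which this graph does not otherwise use.
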(event Custom|MoveGate
  (Utilities|FlowControl|FlipFlop
    (:A
      (bind _newtrack_0 (Timeline|Timeline_0 PlayFromStart)
        (:Update
          (Transformation|SetRelativeLocation (Variables|Debug|GetStaticMeshComponent) (Math|Vector|MakeVector 1.7e+03 3.4e+03 _newtrack_0) false false))))
    (:B
      (bind _newtrack_0_2 (Timeline|Timeline_1 PlayFromStart)
        (:Update
          (Transformation|SetRelativeLocation (Variables|Debug|GetStaticMeshComponent) (Math|Vector|MakeVector 1.7e+03 3.4e+03 _newtrack_0_2) false false))))))

(event EventBeginPlay
  (bind _ashero_game_mode (Utilities|Casting|CastToHeroGameMode (Game|GetGameMode)))
  (Variables|Default|SetAs%20Hero%20Game%20Mode _ashero_game_mode))

(fn ConstructionScript)