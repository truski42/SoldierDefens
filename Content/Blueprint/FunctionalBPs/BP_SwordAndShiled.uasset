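; Sword and shield pickup item that equips the player's hero and raises their strength.
; On Pickup it casts the player character to Hero_BP2 and, if that hero is overlapping an item, sets the sword-and-shield flag, adds to Strenght and destroys itself.
; SetCorrectItemName writes the item's display name into the widget passed to it.
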(event EventBeginPlay)

(event Collision|EventActorBeginOverlap
  (params (OtherActor :type Actor%20Object%20Reference))
  (|CallParentFunction OtherActor) ; This node is disabled and will not be called.\nDrag off pins to build functionality.
)

(event EventTick
  (params (DeltaSeconds :type Float%20%28single-precision%29)))

(event EventSetCorrectItemName
  (params (Widget%20Reference :type WBP%20Equip%20Item%20Prompt%20Object%20Reference))
  (Variables|/Game/Blueprint/Widget/PlayerWidgets/WBP_EquipItemPrompt.WBP_EquipItemPrompt_C|SetItemName Widget%20Reference "Sword&Shield"))

(event EventPickup
  (bind _ashero_bp2 (Utilities|Casting|CastToHero_BP2 (Game|GetPlayerCharacter 0)))
  (if (Variables|/Script/Soldier.Hero|GetbIsOverlappingItem _ashero_bp2)
    (Variables|/Script/Soldier.Hero|SetbHasSwordandShield _ashero_bp2 true)
    (Variables|/Script/Soldier.Hero|SetStrenght _ashero_bp2 (+ (Variables|/Script/Soldier.Hero|GetStrenght _ashero_bp2) 5.0))
    (Actor|DestroyActor)))

(fn ConstructionScript
  (|CallParentFunction))