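; BP_Item is an item actor that shows an equip prompt when the Hero_BP2 character overlaps its interaction box.
; Overlap begin sets the hero's IsOverlappingItem flag, creates a WBP_EquipItemPrompt and passes it to SetCorrectItemName before display.
; Overlap end clears the flag and removes every top-level prompt widget of that class.
; SetCorrectItemName is an empty stub, and Pickup only prints a placeholder message.
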(event OnComponentBeginOverlap(InteractCollisionBox)
  (params (OverlappedComponent :type Primitive%20Component%20Object%20Reference) (OtherActor :type Actor%20Object%20Reference) (OtherComp :type Primitive%20Component%20Object%20Reference) (OtherBodyIndex :type Integer) (bFromSweep :type Boolean) (SweepResult :type Hit%20Result%20Structure%20%28by%20ref%29))
  (bind _ashero_bp2 (Utilities|Casting|CastToHero_BP2 OtherActor))
  (Variables|/Script/Soldier.Hero|SetbIsOverlappingItem _ashero_bp2 true)
  (bind _returnvalue (UserInterface|CreateWidget "/Game/Blueprint/Widget/PlayerWidgets/WBP_EquipItemPrompt.WBP_EquipItemPrompt_C"))
  (CallFunction|SetCorrectItemName _returnvalue)
  (UserInterface|Viewport|AddtoViewport _returnvalue 0))

(event OnComponentEndOverlap(InteractCollisionBox)
  (params (OverlappedComponent :type Primitive%20Component%20Object%20Reference) (OtherActor :type Actor%20Object%20Reference) (OtherComp :type Primitive%20Component%20Object%20Reference) (OtherBodyIndex :type Integer))
  (bind _ashero_bp2 (Utilities|Casting|CastToHero_BP2 OtherActor))
  (Variables|/Script/Soldier.Hero|SetbIsOverlappingItem _ashero_bp2 false)
  (bind _foundwidgets (Widget|GetAllWidgetsOfClass "/Game/Blueprint/Widget/PlayerWidgets/WBP_EquipItemPrompt.WBP_EquipItemPrompt_C" true))
  (for _array_element _foundwidgets
    (Widget|RemovefromParent _array_element)))

(event Custom|Pickup_1_1)

(event EventPickup
  (Development|PrintString "Hello"))

(fn ConstructionScript)

(fn SetCorrectItemName
  (params (Widget%20Reference :type WBP%20Equip%20Item%20Prompt%20Object%20Reference)))