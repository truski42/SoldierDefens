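; RandomSpawnItems is a spawner actor that places a sword-and-shield pickup or item in the level at its own transform.
; On BeginPlay it binds SpawnItem to the HeroGameMode sword-and-shield spawn event, so the game mode decides when BP_SwordAndShiled spawns.
; Despite the name, nothing is random at runtime: the child-actor class swap and random yaw rotation are disconnected.
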(event Custom|SpawnItem
  ;[1 1 1] Spawn Actor
  (Game|SpawnActorfromClass "/Game/Blueprint/FunctionalBPs/BP_SwordAndShiled.BP_SwordAndShiled_C" (Transformation|GetActorTransform) "Undefined" 0 0))

(event EventBeginPlay
  ;[1 1 1] Spawn Actor
  (bind _ashero_game_mode (Utilities|Casting|CastToHeroGameMode (Game|GetGameMode)))
  (EventDispatchers|BindEventtoSpawnSwordandShield _ashero_game_mode (delegate Custom|SpawnItem)))

(fn ConstructionScript)