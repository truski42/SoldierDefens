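; Game mode that runs wave-based enemy combat, starting with one enemy spawned at the first SpawnEnemy actor.
; CheckEnemyLeft advances the wave when no enemies remain, toggles the stairs before and after a timed pause, then calls CallSpawnNextWave.
; MoveStairs forwards to the first Stairs actor, identically whether or not a wave is active.
; Each wave start briefly shows a WBP_WaveInfo widget.
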(event Custom|CheckEnemyLeft
  (bind _wavelevel (Variables|Default|GetWaveLevel))
  (if (== (Variables|Default|GetEnemyAlive) 0)
    (Math|Integer|IncrementInt _wavelevel
      (:%20%20
        (Development|PrintString (Utilities|String|ToString(Integer) _wavelevel))
        (Variables|Default|SetWaveActive false)
        (CallFunction|MoveStairs)
        (Utilities|FlowControl|Delay 5.0)
        (CallFunction|MoveStairs)
        (Default|CallSpawnNextWave)
        (Variables|Default|SetWaveActive true)
        (bind _returnvalue (UserInterface|CreateWidget "/Game/Blueprint/Widget/GameWidgets/WBP_WaveInfo.WBP_WaveInfo_C"))
        (UserInterface|Viewport|AddtoViewport _returnvalue 0)
        (Utilities|FlowControl|Delay 3.5)
        (Widget|RemovefromParent _returnvalue)))))

(event Custom|MoveStairs
  (if (Variables|Default|GetWaveActive)
    (bind _outactors (Actor|GetAllActorsOfClass "/Game/Assets/Stairs.Stairs_C"))
    (Default|MoveStairs (Utilities|Array|Get(acopy) _outactors))
    (else
      (bind _outactors_2 (Actor|GetAllActorsOfClass "/Game/Assets/Stairs.Stairs_C"))
      (Default|MoveStairs (Utilities|Array|Get(acopy) _outactors_2)))))

(event EventBeginPlay
  (bind _outactors (Actor|GetAllActorsOfClass "/Game/Blueprint/AI/SpawnEnemy.SpawnEnemy_C"))
  (Game|SpawnActorfromClass "/Game/Blueprint/AI/Enemy_BP.Enemy_BP_C" (Transformation|GetActorTransform (Utilities|Array|Get(acopy) _outactors)) "Undefined" 0 0)
  (CallFunction|MoveStairs)
  (bind _returnvalue (UserInterface|CreateWidget "/Game/Blueprint/Widget/GameWidgets/WBP_WaveInfo.WBP_WaveInfo_C"))
  (UserInterface|Viewport|AddtoViewport _returnvalue 0)
  (Utilities|FlowControl|Delay 3.5)
  (Widget|RemovefromParent _returnvalue))

(fn ConstructionScript)