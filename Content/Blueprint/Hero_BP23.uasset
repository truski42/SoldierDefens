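; Hero character Blueprint that adds ledge climbing and melee punching.
; Sphere traces each Tick find the wall and ledge top; near pelvis height, the hero snaps to a paused hang montage, then climbs up or drops on input.
; Attacks need stamina, play a random punch montage and poll a capsule trace on the matching hand until it hits a pawn or the attack ends.
; Health-based death logic is present but unconnected.
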(event Custom|Hang
  (bind _wallnormal (Variables|Default|GetWallNormal))
  (bind _walllocation (Variables|Default|GetWallLocation))
  (bind _returnvalue (* _wallnormal "25.000000,25.000000,25.000000"))
  (bind _returnvalue_2 (+ _returnvalue _walllocation))
  ;[1 1 1] Hang
  (Animation|Montage|PlayMontage (Variables|Character|GetMesh) "/Game/Characters/Soldier/NewSoldier/Hanging_Idle__1__Anim_MontageSoldier2.Hanging_Idle__1__Anim_MontageSoldier2"
    (:then
      (Class|AnimInstance|MontagePause (Components|SkeletalMesh|GetAnimInstance (Variables|Character|GetMesh)) "/Game/Characters/Soldier/NewSoldier/Hanging_Idle__1__Anim_MontageSoldier2.Hanging_Idle__1__Anim_MontageSoldier2")
      (Variables|Default|SetisClimbing true)
      (Components|MoveComponentTo (Variables|Default|GetCapsuleComponent) (Math|Vector|MakeVector (.x _returnvalue_2) (.y _returnvalue_2) (- (.z (Variables|Default|GetHeightLocation)) 1.2e+02)) (Math|Rotator|MakeRotfromX (* _wallnormal "-1.000000,-1.000000,-1.000000")) true true 0.2 false))))

(event Custom|DropDown
  ;[1 1 1] Climbing
  (Variables|Default|SetisClimbing false)
  (Pawn|Components|CharacterMovement|SetMovementMode (Variables|Character|GetCharacterMovement) "MOVE_Falling" 0)
  (Animation|StopAnimMontage "/Game/Characters/Soldier/NewSoldier/Hanging_Idle__1__Anim_MontageSoldier2.Hanging_Idle__1__Anim_MontageSoldier2"))

(event Custom|ClimbUp
  (bind _returnvalue (Transformation|GetActorForwardVector))
  ;[1 1 1] Climbing
  (Animation|Montage|PlayMontage (Variables|Character|GetMesh) "/Game/Characters/Soldier/NewSoldier/Climbing_Anim_MontageSoldier2.Climbing_Anim_MontageSoldier2"
    (:OnNotifyBegin
      (Components|MoveComponentTo (Variables|Default|GetCapsuleComponent) (+ (Transformation|GetWorldLocation (Variables|Default|GetCapsuleComponent)) (* _returnvalue "50.000000,50.000000,50.000000")) (Math|Rotator|MakeRotfromX _returnvalue) true true 0.2 false)
      (Variables|Default|SetisClimbing false)
      (CallFunction|FinishingClimbing)
      (Pawn|Components|CharacterMovement|SetMovementMode (Variables|Character|GetCharacterMovement) "MOVE_Walking" 0))))

(event Custom|PunchTrace
  (bind _mesh (Variables|Character|GetMesh))
  (bind _lefthand_ (Variables|Default|GetLeftHand?))
  (bind _returnvalue (select _lefthand_ "hand_l" "hand_r"))
  (bind _returnvalue_2 (Transformation|GetSocketLocation _mesh _returnvalue))
  (if (Variables|Default|GetisAttacking)
    (bind (_outhit _returnvalue_3) (Class|KismetSystemLibrary|CapsuleTraceSingleforObjects 0 _returnvalue_2 _returnvalue_2 2e+01 0.0 (Utilities|Array|MakeArray "ObjectTypeQuery3") false 0 "ForDuration" true))
    (if _returnvalue_3
      (bind _asenemy_bp (Utilities|Casting|CastTo (.HitActor (Collision|BreakHitResult _outhit))))
      (CallFunction|Hit _asenemy_bp)
      (else
        (Utilities|FlowControl|Delay 0 0.01)
        (CallFunction|PunchTrace)))))

(event Custom|FinishingClimbing
  ;[1 1 1] Climbing
  (Utilities|FlowControl|DoOnce false) ; enters at Reset
)

(event EventBeginPlay)

(event EventTick
  (params (DeltaSeconds :type Float%20%28single-precision%29))
  (CallFunction|ForwardForce)
  (CallFunction|HeightForce))

(event Input|ActionEvents|InputActionClimbUp
  (params (Key :type Key%20Structure :default "None"))
  ;[1 1 1] Climbing
  (:Pressed
    (if (Variables|Default|GetisClimbing)
      (Utilities|FlowControl|DoOnce false
        (:Completed
          (CallFunction|ClimbUp))))))

(event Input|ActionEvents|InputActionDropDown
  (params (Key :type Key%20Structure :default "None"))
  ;[1 1 1] Climbing
  (:Pressed
    (if (Variables|Default|GetisClimbing)
      (CallFunction|DropDown))))

(event Input|ActionEvents|InputActionAttack
  (params (Key :type Key%20Structure :default "None"))
  (bind _charactermovement (Variables|Character|GetCharacterMovement))
  ;[1 1 1] Attack
  (:Pressed
    (if (> (Variables|Default|GetcurrentStamina) 0.15)
      (if (and (not (AI|Components|NavMovement|IsFalling (Variables|Character|GetCharacterMovement))) (not (Variables|Default|GetisAttacking)))
        (Variables|Default|SetisAttacking true)
        (bind _output_get (Variables|Default|SetNewVar_0 (Utilities|Array|Get(acopy) (Variables|Default|GetPunchMontage) (Math|Random|RandomIntegerinRange 0 1))))
        (Variables|Default|SetLeftHand? (Utilities|String|Contains (Utilities|GetDisplayName _output_get) "left"))
        (Pawn|Components|CharacterMovement|DisableMovement _charactermovement)
        (bind _returnvalue (Animation|PlayAnimMontage _output_get 1.0 "None"))
        (Utilities|FlowControl|Sequence
          (:then_0
            (Utilities|FlowControl|Delay 0 _returnvalue)
            (Pawn|Components|CharacterMovement|SetMovementMode _charactermovement "MOVE_Walking" 0)
            (Variables|Default|SetisAttacking false))
          (:then_1
            (CallFunction|PunchTrace)))))))

(fn ConstructionScript)

(fn ForwardForce
  (bind _returnvalue (Transformation|GetActorLocation))
  (bind _outhit (Collision|SphereTraceByChannel 0 _returnvalue (+ _returnvalue (* (Transformation|GetActorForwardVector) "150.000000,150.000000,150.000000")) 1e+01 "TraceTypeQuery3" false 0 "ForOneFrame"))
  (Variables|Default|SetWallNormal (.normal _outhit))
  (Variables|Default|SetWallLocation (.location _outhit)))

(fn HeightForce
  (bind _returnvalue (Transformation|GetActorLocation))
  (bind _returnvalue_2 (Transformation|GetActorForwardVector))
  (bind _charactermovement (Variables|Character|GetCharacterMovement))
  (bind _returnvalue_3 (* _returnvalue_2 "75.000000,75.000000,75.000000"))
  (bind _returnvalue_4 (+ _returnvalue "0,0,500.000000" _returnvalue_3))
  (bind (_outhit _returnvalue_5) (Collision|SphereTraceByChannel 0 _returnvalue_4 (- _returnvalue_4 "0,0,500.000000") 1e+01 "TraceTypeQuery3" false 0 "ForOneFrame"))
  (if _returnvalue_5
    (Variables|Default|SetHeightLocation (.location _outhit))
    (if (Math|Float|InRange(Float) (- (.z (Transformation|GetSocketLocation (Variables|Character|GetMesh) "PelvisSocket")) (.Z (Math|Vector|BreakVector (.location _outhit)))) -2e+01 1.0)
      (if (not (Variables|Default|GetisClimbing))
        (Pawn|Components|CharacterMovement|SetMovementMode _charactermovement "MOVE_Flying" 0)
        (Components|Movement|StopMovementImmediately _charactermovement)
        (CallFunction|Hang)))))

(fn IsBetween
  (params (Value :type Float%20%28double-precision%29) (Min :type Float%20%28double-precision%29) (Max :type Float%20%28double-precision%29))
  (if (> Value Min)
    (if (< Value Max)
      (return true)
      (else
        (return false)))
    (else
      (return false))))