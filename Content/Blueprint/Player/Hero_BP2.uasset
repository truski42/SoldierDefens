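; Player hero character with ledge climbing, melee combat, blocking, item interaction and an inventory screen.
; Tick runs wall and ledge sphere traces that trigger hanging, and applies the paladin mesh and animations when armed.
; Stamina-gated attacks play montages while capsule traces recurse until they hit an enemy.
; Hits play block or impact montages, then apply the first found enemy's strength as damage; an overlap box collects lock-on candidates.
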(event OnComponentBeginOverlap(TargetCollisionBox)
  (params (OverlappedComponent :type Primitive%20Component%20Object%20Reference) (OtherActor :type Actor%20Object%20Reference) (OtherComp :type Primitive%20Component%20Object%20Reference) (OtherBodyIndex :type Integer) (bFromSweep :type Boolean) (SweepResult :type Hit%20Result%20Structure%20%28by%20ref%29))
  ;[1 1 1] Targeting/Locking
  (bind _asenemy_bp (Utilities|Casting|CastToEnemy_BP OtherActor))
  (Utilities|Array|AddUnique (Variables|Default|GetlockOnCandidates) _asenemy_bp))

(event OnComponentEndOverlap(TargetCollisionBox)
  (params (OverlappedComponent :type Primitive%20Component%20Object%20Reference) (OtherActor :type Actor%20Object%20Reference) (OtherComp :type Primitive%20Component%20Object%20Reference) (OtherBodyIndex :type Integer))
  ;[1 1 1] Targeting/Locking
  (bind _asenemy_bp (Utilities|Casting|CastToEnemy_BP OtherActor))
  (Utilities|Array|RemoveItem (Variables|Default|GetlockOnCandidates) _asenemy_bp))

(event Custom|Hit
  (bind _bhasswordandshield (Variables|Default|GetbHasSwordandShield))
  ;[1 1 1] Player Hit Event
  (Utilities|FlowControl|DoOnce false :!label _label
    (:Completed
      (if (Variables|Default|GetisBlocking)
        (if _bhasswordandshield
          (|ImpactAnimationWithShield_2 :!label _label_2
            (:else
              _))
          (else
            (|ImpactAnimationWithHands :!label _label_3
              (:else
                _))))
        (Development|PrintString (Utilities|String|ToString(Float) (Variables|Default|GetHealth)))
        (goto _label Reset)
        (elif _bhasswordandshield
          (goto _label_2 execute2)
          (else
            (goto _label_3 execute2)))))))

(event Custom|DropDown
  ;[1 1 1] Climbing
  (Variables|Default|SetisClimbing false)
  (Pawn|Components|CharacterMovement|SetMovementMode (Variables|Character|GetCharacterMovement) "MOVE_Falling" 0)
  (Animation|StopAnimMontage "/Game/Characters/Soldier/NewSoldier/Hanging_Idle__1__Anim_MontageSoldier2.Hanging_Idle__1__Anim_MontageSoldier2"))

(event Custom|ClimbUp
  (bind _returnvalue (Transformation|GetActorForwardVector))
  ;[1 1 1] Climbing
  (Animation|Montage|PlayMontage (Variables|Character|GetMesh) "/Game/Characters/Soldier/NewSoldier/Climbing_Anim_MontageSoldier2.Climbing_Anim_MontageSoldier2"
    (:OnNotifyBegin
      (Components|MoveComponentTo (Variables|Default|GetCapsuleComponent) (+ (Transformation|GetWorldLocation (Variables|Default|GetCapsuleComponent)) (* _returnvalue "50.000000,50.000000,50.000000")) (Math|Rotator|MakeRotfromX _returnvalue) true true 0.2 false)
      (Variables|Default|SetisClimbing false)
      (CallFunction|FinishingClimbing)
      (Pawn|Components|CharacterMovement|SetMovementMode (Variables|Character|GetCharacterMovement) "MOVE_Walking" 0))))

(event Custom|PunchTraceSword
  (bind _mesh (Variables|Character|GetMesh))
  ;[1 1 1] Punch line trace with sword
  (if (Variables|Default|GetisAttacking)
    (bind (_outhit _returnvalue) (Class|KismetSystemLibrary|CapsuleTraceSingleforObjects (Transformation|GetSocketLocation _mesh "StartSwordSocket") (Transformation|GetSocketLocation _mesh "EndSwordSocket") 2e+01 0.0 (Utilities|Array|MakeArray "ObjectTypeQuery3") false 0 "ForDuration" true))
    (if _returnvalue
      (bind _asenemy_bp (Utilities|Casting|CastToEnemy_BP (.HitActor (Collision|BreakHitResult _outhit))))
      (Default|Hit _asenemy_bp)
      (else
        (Utilities|FlowControl|Delay 0.01)
        (CallFunction|PunchTraceSword)))))

(event Custom|FinishingClimbing
  ;[1 1 1] Climbing
  (Utilities|FlowControl|DoOnce false) ; enters at Reset
)

(event Custom|Hang
  (bind _wallnormal (Variables|Default|GetWallNormal))
  (bind _walllocation (Variables|Default|GetWallLocation))
  (bind _returnvalue (* _wallnormal "25.000000,25.000000,25.000000"))
  (bind _returnvalue_2 (+ _returnvalue _walllocation))
  ;[1 1 1] Hang
  (Animation|Montage|PlayMontage (Variables|Character|GetMesh) "/Game/Characters/Soldier/NewSoldier/Hanging_Idle__1__Anim_MontageSoldier2.Hanging_Idle__1__Anim_MontageSoldier2"
    (:then
      (Class|AnimInstance|MontagePause (Components|SkeletalMesh|GetAnimInstance (Variables|Character|GetMesh)) "/Game/Characters/Soldier/NewSoldier/Hanging_Idle__1__Anim_MontageSoldier2.Hanging_Idle__1__Anim_MontageSoldier2")
      (Variables|Default|SetisClimbing true)
      (Components|MoveComponentTo (Variables|Default|GetCapsuleComponent) (Math|Vector|MakeVector (.x _returnvalue_2) (.y _returnvalue_2) (- (.z (Variables|Default|GetHeightLocation)) 1.2e+02)) (Math|Rotator|MakeRotfromX (* _wallnormal "-1.000000,-1.000000,-1.000000")) true true 0.2 false))))

(event Custom|PunchTraceHands
  (bind _mesh (Variables|Character|GetMesh))
  (bind _lefthand_ (Variables|Default|GetLeftHand?))
  (bind _returnvalue (select _lefthand_ "hand_l" "hand_r"))
  (bind _returnvalue_2 (Transformation|GetSocketLocation _mesh _returnvalue))
  ;[1 1 1] Punch line trace with hands
  (if (Variables|Default|GetisAttacking)
    (bind (_outhit _returnvalue_3) (Class|KismetSystemLibrary|CapsuleTraceSingleforObjects _returnvalue_2 _returnvalue_2 2e+01 0.0 (Utilities|Array|MakeArray "ObjectTypeQuery3") false 0 "ForDuration" true))
    (if _returnvalue_3
      (bind _asenemy_bp (Utilities|Casting|CastToEnemy_BP (.HitActor (Collision|BreakHitResult _outhit))))
      (Default|Hit _asenemy_bp)
      (else
        (Utilities|FlowControl|Delay 0.01)
        (CallFunction|PunchTraceHands)))))

(event EventBeginPlay
  (bind _asenemy_bp (Utilities|Casting|CastToEnemy_BP (Game|GetPlayerCharacter 0)))
  (Variables|Default|SetAs%20Enemy%20BP _asenemy_bp))

(event EventToggleLockonEffect
  ;[1 1 1] Indicator
  (bind _lockedonactor (Variables|Default|GetlockedOnActor)
    (:then
      (bind _lockonindicatorref (Variables|Default|GetLockOnIndicatorRef)
        (:then
          (Actor|DestroyActor _lockonindicatorref))
        (:else
          _))
      (bind _returnvalue (Game|SpawnActorfromClass "/Game/Blueprint/AI/LockIndicator.LockIndicator_C" (Transformation|GetActorTransform _lockedonactor) "Undefined" 0 0))
      (Actor|DestroyActor _returnvalue))
    (:else
      (bind _lockonindicatorref_2 (Variables|Default|GetLockOnIndicatorRef)
        (:then
          (Actor|DestroyActor _lockonindicatorref_2))
        (:else)))))

(event EventTick
  (params (DeltaSeconds :type Float%20%28single-precision%29))
  (bind _mesh (Variables|Character|GetMesh))
  (CallFunction|ForwardForce)
  (CallFunction|HeightForce)
  (if (Variables|Default|GetbHasSwordandShield)
    (Class|SkinnedMeshComponent|SetSkeletalMesh _mesh "/Game/Characters/Soldier/SoliderWithSword/Paladin_WProp_J_Nordstrom__1_.Paladin_WProp_J_Nordstrom__1_" false)
    (Class|SkeletalMeshComponent|SetAnimClass _mesh "/Game/Characters/Soldier/SoliderWithSword/Animation_SoliderWithSword_Shield.Animation_SoliderWithSword_Shield_C")))

(event Input|ActionEvents|InputActionClimbUp
  (params (Key :type Key%20Structure :default "None"))
  ;[1 1 1] Climbing
  (:Pressed
    (if (Variables|Default|GetisClimbing)
      (Utilities|FlowControl|DoOnce false
        (:Completed
          (CallFunction|ClimbUp))))))

(event Input|ActionEvents|InputActionDropDown
  (params (Key :type Key%20Structure :default "None"))
  ;[1 1 1] Climbing
  (:Pressed
    (if (Variables|Default|GetisClimbing)
      (CallFunction|DropDown))))

(event Input|ActionEvents|InputActionAttack
  (params (Key :type Key%20Structure :default "None"))
  (bind _charactermovement (Variables|Character|GetCharacterMovement))
  ;[1 1 1] Attack
  (:Pressed
    (if (> (Variables|Default|GetcurrentStamina) 0.15)
      (if (not (AI|Components|NavMovement|IsCrouching _charactermovement))
        (if (and (not (AI|Components|NavMovement|IsFalling _charactermovement)) (not (Variables|Default|GetisAttacking)))
          (Variables|Default|SetisAttacking true)
          (if (Variables|Default|GetbHasSwordandShield)
            (|AttackAnimationWithSword)
            (else
              (|AttackAnimationWithHands))))))))

(event Input|ActionEvents|InputActionBlock
  (params (Key :type Key%20Structure :default "None"))
  ;[1 1 1] Blocking
  (:Pressed
    (Class|Hero|StartBlocking))
  (:Released
    (Class|Hero|StopBlocking)))

(event Input|ActionEvents|InputActionEquip
  (params (Key :type Key%20Structure :default "None"))
  ;[1 1 1] Pickup interace
  (:Pressed
    (for _array_element (Collision|GetOverlappingActors "/Game/Blueprint/FunctionalBPs/BP_Item.BP_Item_C" :!class /Script/Engine.Actor)
      (if (Utilities|DoesObjectImplementInterface _array_element "/Game/Blueprint/FunctionalBPs/PickupInterface.PickupInterface_C")
        (Class|PickupInterface|Pickup(Message) _array_element)))))

(event Input|ActionEvents|InputActionInventory
  (params (Key :type Key%20Structure :default "None"))
  (bind _returnvalue (Game|GetPlayerController 0))
  (:Pressed
    (Utilities|FlowControl|FlipFlop
      (:A
        (Game|Player|SetViewTargetwithBlend (Game|GetPlayerController 0) (Variables|/Script/Engine.ChildActorComponent|GetChildActor (Variables|Default|GetInventoryCamera)) 0.5 "VTBlend_Linear" 0.0 false)
        (bind _returnvalue_2 (UserInterface|CreateWidget "/Game/Blueprint/Widget/PlayerWidgets/WBP_PlayerInventory.WBP_PlayerInventory_C" 0 0))
        (UserInterface|Viewport|AddtoViewport _returnvalue_2 0)
        (Input|SetInputModeUIOnly _returnvalue 0 "DoNotLock")
        (Variables|/Script/Engine.PlayerController|SetbShowMouseCursor _returnvalue true)))))

(event Input|ActionEvents|InputActionInteract
  (params (Key :type Key%20Structure :default "None"))
  ;[1 1 1] Interact with actor
  (:Pressed
    (bind _array_element (Utilities|Array|ForEachLoopwithBreak (Collision|GetOverlappingActors "/Script/Engine.Actor" :!class /Script/Engine.Actor) :!label _label)
      (:LoopBody
        (if (Utilities|DoesObjectImplementInterface _array_element "/Game/Blueprint/FunctionalBPs/InteractInterface.InteractInterface_C")
          (Class|InteractInterface|Interact(Message) _array_element)
          (goto _label Break))))))

(fn ConstructionScript)

(fn ForwardForce
  (bind _returnvalue (Transformation|GetActorLocation))
  (bind _outhit (Collision|SphereTraceByChannel _returnvalue (+ _returnvalue (* (Transformation|GetActorForwardVector) "150.000000,150.000000,150.000000")) 1e+01 "TraceTypeQuery3" false 0 "None"))
  (Variables|Default|SetWallNormal (.normal _outhit))
  (Variables|Default|SetWallLocation (.location _outhit)))

(fn HeightForce
  (bind _returnvalue (Transformation|GetActorLocation))
  (bind _returnvalue_2 (Transformation|GetActorForwardVector))
  (bind _charactermovement (Variables|Character|GetCharacterMovement))
  (bind _returnvalue_3 (* _returnvalue_2 "75.000000,75.000000,75.000000"))
  (bind _returnvalue_4 (+ _returnvalue "0,0,500.000000" _returnvalue_3))
  (bind (_outhit _returnvalue_5) (Collision|SphereTraceByChannel _returnvalue_4 (- _returnvalue_4 "0,0,500.000000") 1e+01 "TraceTypeQuery3" false 0 "None"))
  (if _returnvalue_5
    (Variables|Default|SetHeightLocation (.location _outhit))
    (if (Math|Float|InRange(Float) (- (.z (Transformation|GetSocketLocation (Variables|Character|GetMesh) "PelvisSocket")) (.Z (Math|Vector|BreakVector (.location _outhit)))) -2e+01 1.0)
      (if (not (Variables|Default|GetisClimbing))
        (Pawn|Components|CharacterMovement|SetMovementMode _charactermovement "MOVE_Flying" 0)
        (Components|Movement|StopMovementImmediately _charactermovement)
        (CallFunction|Hang)))))

(fn IsBetween
  (params (Value :type Float%20%28double-precision%29) (Min :type Float%20%28double-precision%29) (Max :type Float%20%28double-precision%29))
  (if (> Value Min)
    (if (< Value Max)
      (return true)
      (else
        (return false)))
    (else
      (return false))))