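; BP_Inventory is a player inventory Blueprint that tracks item quantities by ID in InventoryMap.
; AddToInventory looks up the ItemID, then either adds the incoming quantity to the stored value or creates a new entry, with no limit checks.
; The event graph holds only a disabled BeginPlay, and the file contains no removal logic.
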(event EventBeginPlay)

(fn AddtoInventory
  (params (Item%20ID :type Integer) (Quantity :type Integer))
  (bind _inventorymap (Variables|Default|GetInventoryMap))
  (bind (_value _returnvalue) (Utilities|Map|Find _inventorymap Item%20ID))
  (if _returnvalue
    (Utilities|Map|Add (Variables|Default|GetInventoryMap) Item%20ID (+ Quantity _value))
    (return)
    (else
      (Utilities|Map|Add (Variables|Default|GetInventoryMap) Item%20ID Quantity))))