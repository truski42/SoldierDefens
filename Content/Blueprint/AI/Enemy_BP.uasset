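; Melee enemy character for a wave-based mode, with level, health and strength scaled from the hero's level and current wave.
; Pawn sensing flags the player in the blackboard, and overlapping the attack box plays a random punch with a recursively polled hand-socket capsule trace.
; Hits play a block montage, apply damage and update the health widget.
; Death grants experience, updates the game mode's enemy count and may drop loot.
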(event OnSeePawn(PawnSensing)
  (params (Pawn :type Pawn%20Object%20Reference))
  (Utilities|Casting|CastToHero_BP2 Pawn)
  (AI|Components|Blackboard|SetValueasBool (AI|GetBlackboard (AI|GetAIController self)) (Utilities|Name|MakeLiteralName "hasSeenPlayer?") true))

(event OnComponentBeginOverlap(EnemyAttackCollisionBox)
  (params (OverlappedComponent :type Primitive%20Component%20Object%20Reference) (OtherActor :type Actor%20Object%20Reference) (OtherComp :type Primitive%20Component%20Object%20Reference) (OtherBodyIndex :type Integer) (bFromSweep :type Boolean) (SweepResult :type Hit%20Result%20Structure%20%28by%20ref%29))
  (bind _returnvalue (Math|Random|RandomIntegerinRange 0 1))
  (bind _punchmontage (Variables|Default|GetPunchMontage))
  (bind _output (Utilities|Array|Get(acopy) _punchmontage _returnvalue))
  ;[1 1 1] Player overlap in collsionbox
  (Utilities|Casting|CastToHero_BP2 OtherActor)
  (if (and (not (AI|Components|NavMovement|IsFalling (Variables|Character|GetCharacterMovement))) (not (Variables|/Script/Soldier.Hero|GetisAttacking (Variables|Default|GetAs%20Hero%20BP2))))
    (Variables|Default|SetisAttacking true)
    (bind _output_get (Variables|Default|SetSetCurrentAnimation _output))
    (Variables|Default|SetLeftHand? (Utilities|String|Contains (Utilities|GetDisplayName _output) "left"))
    (bind _returnvalue_2 (Animation|PlayAnimMontage _output_get 1.0 "None"))
    (Utilities|FlowControl|Sequence
      (:then_0
        (Utilities|FlowControl|Delay _returnvalue_2)
        (Variables|Default|SetisAttacking false))
      (:then_1
        (CallFunction|PunchTrace)))))

(event OnComponentEndOverlap(EnemyAttackCollisionBox)
  (params (OverlappedComponent :type Primitive%20Component%20Object%20Reference) (OtherActor :type Actor%20Object%20Reference) (OtherComp :type Primitive%20Component%20Object%20Reference) (OtherBodyIndex :type Integer))
  ;[1 1 1] Player overlap in collsionbox
  (Utilities|Casting|CastToHero_BP2 OtherActor)
  (Utilities|FlowControl|Delay 1.0)
  (Variables|Default|SetisAttacking false))

(event Custom|Hit
  (bind _returnvalue (Transformation|GetActorLocation))
  ;[1 1 1] Enemy is hitting by player
  (Utilities|FlowControl|DoOnce false :!label _label
    (:Completed
      (Audio|PlaySoundatLocation "/Game/Sounds/Melee/PunchCue.PunchCue" (Transformation|GetActorLocation) "0, 0, 0" 1.0 1.0 0.0 0 0 0 0)
      (bind _returnvalue_2 (Animation|PlayAnimMontage (select (Variables|/Game/Blueprint/Player/Hero_BP2.Hero_BP2_C|GetLeftHand? (Variables|Default|GetAs%20Hero%20BP2)) "/Game/Characters/Soldier/NewSoldier/Attack-Block/Right_Block_Anim_Montage.Right_Block_Anim_Montage" "/Game/Characters/Soldier/NewSoldier/Attack-Block/Left_Block_Anim_Montage.Left_Block_Anim_Montage") 1.0 "None"))
      (Utilities|FlowControl|Delay _returnvalue_2)
      (Class|DefaultEnemy|TakeDamage (Variables|/Script/Soldier.Hero|GetStrenght (Variables|Default|GetAs%20Hero%20BP2)))
      (CallFunction|HealthBarProgrees)
      (if (< (Variables|Default|GetHealth) 0.0)
        (Class|Hero|GainExperience (Variables|Default|GetAs%20Hero%20BP2) (Variables|Default|GetexpWorth))
        (Pawn|Components|CharacterMovement|DisableMovement (Variables|Character|GetCharacterMovement))
        (Collision|SetCollisionEnabled (Variables|Default|GetCapsuleComponent) "NoCollision")
        (bind _returnvalue_3 (Animation|PlayAnimMontage "/Game/Characters/Soldier/NewSoldier/Sword_And_Shield_Death_Anim_Montage.Sword_And_Shield_Death_Anim_Montage" 1.0 "None"))
        (Utilities|FlowControl|Delay (- _returnvalue_3 0.3))
        (Actor|DestroyActor)
        (bind _ashero_game_mode (Utilities|Casting|CastToHeroGameMode (Game|GetGameMode)))
        (Math|Integer|DecrementInt (Variables|/Script/Soldier.Hero_GameMode|GetEnemyAlive _ashero_game_mode)
          (:%20%20
            (Default|CheckEnemyLeft _ashero_game_mode)
            (if (Math|Random|RandomBoolwithWeight 0.4)
              (bind _outhit (Collision|LineTraceByChannel _returnvalue (- _returnvalue "0,0,1000.000000") "TraceTypeQuery1" false 0 "None"))
              (Game|SpawnActorfromClass "/Game/Blueprint/FunctionalBPs/BP_LootFromEnemy.BP_LootFromEnemy_C" (Math|Transform|MakeTransform (.Location (Collision|BreakHitResult _outhit)) "0, 0, 0" "1.000000,1.000000,1.000000") "Undefined" 0 0))))
        (else
          (goto _label Reset))))))

(event Custom|PunchTrace
  (bind _mesh (Variables|Character|GetMesh))
  (bind _lefthand_ (Variables|Default|GetLeftHand?))
  (bind _returnvalue (select _lefthand_ "hand_l" "hand_r"))
  (bind _returnvalue_2 (Transformation|GetSocketLocation _mesh _returnvalue))
  ;[1 1 1] Punch linetrace
  (if (Variables|Default|GetisAttacking)
    (bind (_outhit _returnvalue_3) (Class|KismetSystemLibrary|CapsuleTraceSingleforObjects _returnvalue_2 _returnvalue_2 2e+01 0.0 (Utilities|Array|MakeArray "ObjectTypeQuery3") false 0 "ForDuration" true))
    (if _returnvalue_3
      (bind _ashero_bp2 (Utilities|Casting|CastToHero_BP2 (.HitActor (Collision|BreakHitResult _outhit))))
      (Default|Hit _ashero_bp2)
      (else
        (Utilities|FlowControl|Delay 0.01)
        (CallFunction|PunchTrace)))))

(event EventBeginPlay
  ;[1 1 1] Start
  (CallFunction|HealthBarProgrees)
  (bind _ashero_bp2 (Utilities|Casting|CastToHero_BP2 (Game|GetPlayerCharacter 0)))
  (Variables|Default|SetAs%20Hero%20BP2 _ashero_bp2)
  (bind _ashero_game_mode (Utilities|Casting|CastToHeroGameMode (Game|GetGameMode)))
  (Variables|Default|SetAs%20Hero%20Game%20Mode _ashero_game_mode)
  (Math|Integer|IncrementInt (Variables|/Script/Soldier.Hero_GameMode|GetEnemyAlive _ashero_game_mode)
    (:%20%20
      (CallFunction|Levelup)
      (Development|PrintString (Utilities|String|ToString(Integer) (Variables|Default|GetEnemyLevel))))))

(fn ConstructionScript)

(fn HealthBarProgrees
  (bind _aswbp_ai_health (Utilities|Casting|CastToWBP_AI_Health (UserInterface|GetUserWidgetObject (Variables|Default|GetHealthBar))))
  (Variables|/Game/Blueprint/AI/WBP_AI_Health.WBP_AI_Health_C|SetHealth _aswbp_ai_health (/ (Variables|Default|GetHealth) (Variables|Default|GetdefaultHealth)))
  (return))

(fn ExpBar)

(fn Levelup
  (bind _as_hero_game_mode (Variables|Default|GetAs%20Hero%20Game%20Mode))
  (bind _wavelevel (Variables|/Script/Soldier.Hero_GameMode|GetWaveLevel _as_hero_game_mode))
  (bind _output_get (Variables|Default|SetEnemyLevel (+ (Variables|/Script/Soldier.Hero|GetcurrentLevel (Variables|Default|GetAs%20Hero%20BP2)) _wavelevel)))
  (bind _output_get_2 (Variables|Default|SetdefaultHealth (Math|Conversions|ToFloat(Integer) (Math|Float|Round (* _output_get _wavelevel)))))
  (Variables|Default|Sethealth _output_get_2)
  (Variables|Default|SetEnemyStrenght (/ (* (Variables|Default|GetEnemyLevel) 2) 2)))