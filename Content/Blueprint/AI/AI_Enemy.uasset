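; AI_Enemy is an enemy actor that takes damage from the player hero.
; When a Hero_BP2 overlaps it while that hero's IsAttacking flag is set, it subtracts Damage from its Health.
; It destroys itself once Health reaches zero or below.
; Damage is applied only when an overlap begins, and the construction script is empty.
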(event Collision|EventActorBeginOverlap
  (params (OtherActor :type Actor%20Object%20Reference))
  (bind _ashero_bp2 (Utilities|Casting|CastToHero_BP2 OtherActor))
  (if (Variables|/Script/Test.Hero|GetisAttacking _ashero_bp2)
    (Variables|Default|SetHealth (- (Variables|Default|GetHealth) (Variables|Default|GetDamage)))
    (if (<= (Variables|Default|GetHealth) 0)
      (Actor|DestroyActor))))

(fn ConstructionScript)