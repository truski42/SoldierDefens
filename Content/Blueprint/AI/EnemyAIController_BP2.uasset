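; Enemy AI controller that runs the BT_AI behavior tree on BeginPlay.
; It also holds Blueprint movement events: RandomRoam repeatedly moves to random reachable points while IsSeesPlayer is false, and Chase moves toward the Player.
; These events are left disconnected: the perception update handler is empty, and the nodes that would cast to Hero_BP2, schedule Chase or start roaming never run.
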(event OnTargetPerceptionUpdated(AIPerception)
  (params (Actor :type Actor%20Object%20Reference) (Stimulus :type AI%20Stimulus%20Structure)))

(event Custom|RandomRoam
  (bind _returnvalue (Pawn|GetControlledPawn))
  (if (not (Variables|Default|GetisSeesPlayer?))
    (AI|AIMoveTo _returnvalue (.RandomLocation (AI|Navigation|GetRandomReachablePointinRadius (Transformation|GetActorLocation _returnvalue) 1.5e+03 0 0)) 0 5.0 false
      (:OnSuccess
        (CallFunction|RandomRoam)))))

(event Custom|Chase
  (AI|AIMoveTo (Pawn|GetControlledPawn) (Transformation|GetActorLocation (Variables|Default|GetPlayer)) 0 5.0 false))

(event EventBeginPlay
  (AI|RunBehaviorTree "/Game/Blueprint/AI/BehaviorTree/BT_AI.BT_AI"))

(fn ConstructionScript)